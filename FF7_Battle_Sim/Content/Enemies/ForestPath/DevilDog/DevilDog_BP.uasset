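; DevilDog_BP is the Devil Dog enemy Blueprint from the Forest Path area, handling its reactions to damage and death.
; Shortly after BeginPlay, it binds handlers to damage, damage-number and death events.
; The damage and death handlers set state flags, while the number handler creates a TEST_CombatNumbers widget.
; That widget receives the damage value and an offset screen position projected from the dog's root location.
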(event `self.ReceiveBeginPlay`
  (`KismetSystemLibrary.Delay` 0.2)
  (add `self.OnDamageEvent` (delegate `DamageTaken`))
  (add `self.DamageTakenNumberEvent` (delegate `SetDamageTaken`))
  (add `self.OnDeathEvent` (delegate `OnDeath`)))

(event `DamageTaken`
  (set `self.TakingDamage` true))

(event `OnDeath`
  (set `self.EnemyDead` true))

(event `SetDamageTaken` :!signature `self.DamageTakenNumberEvent`
  (params (DamageTaken :type Integer))
  (`self.BuildCombatNumbersWidget` self DamageTaken))

(fn `BuildCombatNumbersWidget`
  (params (DevilDogRef :type "/Game/Enemies/ForestPath/DevilDog/DevilDog_BP Object Reference") (DamageTaken :type Integer))
  (bind _returnvalue (`|CreateWidget` "/Game/HUD/CombatUI/TEST_CombatNumbers.TEST_CombatNumbers_C" null DamageTaken (- (`GameplayStatics.ProjectWorldToScreen` (`GameplayStatics.GetPlayerController` 0) (`SceneComponent.K2_GetComponentLocation` (`Actor.RootComponent` DevilDogRef))) (64.0 16.0))))
  (`UserWidget.AddToViewport` _returnvalue 0))

(fn `UserConstructionScript`)