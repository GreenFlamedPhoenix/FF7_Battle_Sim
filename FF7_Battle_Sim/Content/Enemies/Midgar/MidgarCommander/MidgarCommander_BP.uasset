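; Midgar Commander enemy Blueprint that shows floating combat numbers when it takes damage.
; Shortly after BeginPlay it binds damage, damage-number and death events, though only the damage-number handler does anything.
; That handler passes the damage to CreateDamageWidget, which spawns a TEST_CombatNumbers widget at the actor's root location projected to screen space with a fixed offset.
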(event `self.ReceiveBeginPlay`
  (`KismetSystemLibrary.Delay` 0.2)
  (add `self.OnDamageEvent` (delegate `OnDamageEvent_Event_0`))
  (add `self.DamageTakenNumberEvent` (delegate `DamageTakenNumber`))
  (add `self.OnDeathEvent` (delegate `OnDeathEvent_Event_0`)))

(event `OnDamageEvent_Event_0`)

(event `DamageTakenNumber` :!signature `self.DamageTakenNumberEvent`
  (params (DamageTaken :type Integer))
  (`self.CreateDamageWidget` self DamageTaken))

(event `OnDeathEvent_Event_0`)

(fn `CreateDamageWidget`
  (params (inDamage :type Integer))
  (bind _returnvalue (`|CreateWidget` "/Game/HUD/CombatUI/TEST_CombatNumbers.TEST_CombatNumbers_C" null inDamage (- (`GameplayStatics.ProjectWorldToScreen` (`GameplayStatics.GetPlayerController` 0) (`SceneComponent.K2_GetComponentLocation` (`Actor.RootComponent`))) (64.0 16.0))))
  (`UserWidget.AddToViewport` _returnvalue 0))

(fn `UserConstructionScript`)