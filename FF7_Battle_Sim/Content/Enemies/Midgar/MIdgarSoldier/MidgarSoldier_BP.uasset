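; MidgarSoldier_BP is a Midgar soldier enemy that flags when it takes damage or dies.
; Shortly after BeginPlay it binds to its damage and death events, setting a boolean for each.
; Each hit also spawns a test combat-number widget with a fixed damage value at the soldier's projected screen position.
; The damage and death animation functions are empty stubs.
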(event `self.ReceiveBeginPlay`
  (`KismetSystemLibrary.Delay` 0.2)
  (add `self.OnDamageEvent` (delegate `OnDamageEvent_Event_0`))
  (add `self.OnDeathEvent` (delegate `OnDeathEvent_Event_0`)))

(event `OnDamageEvent_Event_0`
  (set `self.bSoldierTookDamage` true)
  (`self.BuildCombatNumbersWidget` self))

(event `OnDeathEvent_Event_0`
  (set `self.bSoldierDied` true))

(fn `BuildCombatNumbersWidget`
  (params (inSoldierRef :type "/Game/Enemies/Midgar/MIdgarSoldier/MidgarSoldier_BP Object Reference"))
  (bind _returnvalue (`|CreateWidget` "/Game/HUD/CombatUI/TEST_CombatNumbers.TEST_CombatNumbers_C" null 75 (- (`GameplayStatics.ProjectWorldToScreen` (`GameplayStatics.GetPlayerController` 0) (`SceneComponent.K2_GetComponentLocation` (`Actor.RootComponent` inSoldierRef))) (64.0 16.0))))
  (`UserWidget.AddToViewport` _returnvalue 0))

(fn `ManageDamageAnimation`)

(fn `ManageDeathAnimation`)

(fn `UserConstructionScript`)