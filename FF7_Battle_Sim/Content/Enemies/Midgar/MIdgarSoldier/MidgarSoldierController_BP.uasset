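; AI controller for the Midgar Soldier enemy that runs its behavior tree and drives an ATB-style action gauge.
; On BeginPlay it waits briefly, caches the possessed soldier, has it calculate its action speed and starts a looping timer.
; Each tick of that timer adds the soldier's speed to the gauge until it reaches the maximum, then flags ReadyForAction and pauses.
; ResetActionTimer clears the gauge and flag and resumes the timer.
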(event `self.ReceiveBeginPlay`
  (`self.RunBehaviorTree` "/Game/Enemies/Midgar/MIdgarSoldier/MidgarSoldierAI/MidgarSoldierTree.MidgarSoldierTree")
  (`KismetSystemLibrary.Delay` 0.75)
  (bind _asmidgar_soldier_bp (cast `/Game/Enemies/Midgar/MIdgarSoldier/MidgarSoldier_BP` (`self.K2_GetPawn`)))
  (bind _output_get (set `self.SoldierRef` _asmidgar_soldier_bp))
  (`MidgarSoldier.CalculateActionSpeed` _output_get)
  (bind _returnvalue (`KismetSystemLibrary.K2_SetTimer` null "IncreaseActionCount" 0.1 true))
  (set `self.MyActionTimer` _returnvalue))

(fn `IncreaseActionCount`
  (if (< (`self.MyCurrentActionTimer`) (`self.MyMaxActionTimer`))
    (set `self.MyCurrentActionTimer` (+ (`self.MyCurrentActionTimer`) (`MidgarSoldier.MyActionSpeed` (`self.SoldierRef`))))
    (else
      (set `self.bReadyForAction` true)
      (`KismetSystemLibrary.K2_PauseTimerHandle` (`self.MyActionTimer`)))))

(fn `ResetActionTimer`
  (set `self.bReadyForAction` false)
  (set `self.MyCurrentActionTimer` 0.0)
  (`KismetSystemLibrary.K2_UnPauseTimerHandle` (`self.MyActionTimer`)))

(fn `UserConstructionScript`)