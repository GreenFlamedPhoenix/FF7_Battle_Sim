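; Cam1_BP is an actor for Area 3 of Section 1, apparently a camera by its name, that follows a tracked character along the world X axis.
; Each Tick, while TrackedCharacter is valid, it moves to that character's X position plus a fixed offset, keeping its own Y, Z, rotation and scale.
; The move is immediate, with no sweep or smoothing, and nothing in these graphs assigns TrackedCharacter.
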(event `self.ReceiveBeginPlay`)

(event `self.ReceiveTick`
  (params (DeltaSeconds :type "Float (single-precision)"))
  (bind _trackedcharacter (`self.TrackedCharacter`))
  (`/Engine/EditorBlueprintResources/StandardMacros.IsValid` _trackedcharacter
    (:`Is Valid`
      (`self.K2_SetActorTransform` (`KismetMathLibrary.MakeTransform` (`KismetMathLibrary.MakeVector` (+ (.x (.location (`self.GetTransform` _trackedcharacter))) 500.0) (.y (.location (`self.GetTransform`))) (.z (.location (`self.GetTransform`)))) (.rotation (`self.GetTransform`)) (.scale (`self.GetTransform`)))))))

(fn `UserConstructionScript`)